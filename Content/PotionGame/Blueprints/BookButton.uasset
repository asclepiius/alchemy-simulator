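; BookButton is a physical push button in the potion game that sinks when actors, intended to be player hands, overlap its box.
; Each tick it checks the box for overlaps and nudges the mesh down, or back up when clear, clamped between zero and ButtonOffset.
; The construction script raises the mesh to ButtonOffset and sizes an arrow to show the travel path.
; The graph only moves the mesh and triggers no other action.
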(event `self.ReceiveTick`
  (params (DeltaSeconds :type "Float (single-precision)"))
  (bind _staticmesh (`self.StaticMesh`))
  (bind _staticmesh_2 (`self.StaticMesh`))
  (bind (_relativelocation_x _relativelocation_y _relativelocation_z) (`KismetMathLibrary.BreakVector` (`SceneComponent.RelativeLocation` _staticmesh)))
  (bind (_relativelocation_x_2 _relativelocation_y_2 _relativelocation_z_2) (`KismetMathLibrary.BreakVector` (`SceneComponent.RelativeLocation` _staticmesh_2)))
  ;[1 1 1] Button Press
  (if (> (`KismetArrayLibrary.Array_Length` (`PrimitiveComponent.GetOverlappingActors` (`self.Box`) null)) 0)
    ;;[1 1 1] If true then the button moves down from its original position
    (`KismetSystemLibrary.MoveComponentTo` _staticmesh_2 (`KismetMathLibrary.MakeVector` 0.0 0.0 (`KismetMathLibrary.FClamp` (- _relativelocation_z_2 1.5) 0.0 (`self.ButtonOffset`))) (struct) false false 0.0001)
    (else
      ;;[1 1 1] If false then the button moves back up to its original position
      (`KismetSystemLibrary.MoveComponentTo` _staticmesh (`KismetMathLibrary.MakeVector` 0.0 0.0 (`KismetMathLibrary.FClamp` (+ _relativelocation_z 1.5) 0.0 (`self.ButtonOffset`))) (struct) false false 0.0001))))

(fn `UserConstructionScript`
  (bind _buttonoffset (`self.ButtonOffset`))
  ;[1 1 1] Sets visable area in the viewport for the path the button will move
  (set `ArrowComponent.ArrowLength` _buttonoffset (`self.Arrow`))
  (`SceneComponent.K2_SetRelativeLocation` (`self.StaticMesh`) (`KismetMathLibrary.MakeVector` 0.0 0.0 _buttonoffset) false false))