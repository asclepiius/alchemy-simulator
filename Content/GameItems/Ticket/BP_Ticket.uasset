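; BP_Ticket is an in-world ticket item that shows a randomly chosen potion type on a widget.
; On BeginPlay it caches the TicketWidget from its Test widget component, then calls SetRandomPotion.
; SetRandomPotion picks a random row name from PotionTypesTable, writes it to the widget's TopText, and stores that text as the ticket's Type string.
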(event `self.ReceiveBeginPlay`
  (bind _asticket_widget (cast `/Game/GameItems/Ticket/TicketWidget` (`WidgetComponent.GetUserWidgetObject` (`self.test`))))
  (set `self.Ticket Widget` _asticket_widget)
  (`self.Set Random Potion`))

(fn `Set Random Potion`
  (locals (NewLocalVar :type Name :default "Water_Potion"))
  (bind _outrownames (`DataTableFunctionLibrary.GetDataTableRowNames` "/Game/GameItems/Potion/PotionTypesTable.PotionTypesTable"))
  (bind _output_get (set `/Game/GameItems/Ticket/TicketWidget.TopText` (`KismetTextLibrary.Conv_NameToText` (`KismetArrayLibrary.Array_Random` _outrownames)) (`self.Ticket Widget`)))
  (set `self.Type` (`KismetTextLibrary.Conv_TextToString` _output_get)))

(fn `UserConstructionScript`)