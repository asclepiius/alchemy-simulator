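; BP_Book is a crafting workstation that transforms a potion when its button is pressed.
; BeginPlay caches Book-method recipes from RecipesTable, mapping row name to first ingredient, and overlap stores the last colliding potion.
; Tick polls PressMe to animate the button down and back up through a DoOnce, calling ButtonPressed at the bottom.
; ButtonPressed reverse-looks up the potion's first tag in that map and passes the matching row name to ChangePotion.
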(event `self.ReceiveBeginPlay`
  ;[1 1 1] Adds Potion to a map if it satisfies the condition of the crafting method being Book
  (bind _outrownames (`DataTableFunctionLibrary.GetDataTableRowNames` "/Game/GameItems/WorkStations/RecipesTable.RecipesTable"))
  (for _array_element _outrownames
    (bind _returnvalue (`|GetDataTableRow` "/Game/GameItems/WorkStations/RecipesTable.RecipesTable" _array_element)
      (:`then`
        (bind (_crafting_ingredient_1 _crafting_ingredient_2 _crafting_ingredient_3 _method) (break `/Game/GameItems/WorkStations/RecipesStruct` _returnvalue))
        (if (== _method "Book")
          (`BlueprintMapLibrary.Map_Add` (`self.Book Recipies`) _array_element _crafting_ingredient_1))))))

(event `self.ReceiveActorBeginOverlap`
  (params (OtherActor :type "Actor Object Reference"))
  ;[1 1 1] Checks for a collision with book
  (`/Engine/EditorBlueprintResources/StandardMacros.IsValid` OtherActor
    (:`Is Valid`
      (bind _aspotion (cast `/Game/GameItems/Potion/Potion` OtherActor))
      ;;[1 1 1] Finds the type of potion that has collided
      (bind _output_get (set `self.Collided potion` _aspotion))
      (`KismetSystemLibrary.PrintText` (`KismetTextLibrary.Conv_NameToText` (`/Game/GameItems/Potion/Potion.Type` _output_get))))))

(event `self.ReceiveTick`
  (params (DeltaSeconds :type "Float (single-precision)"))
  (bind _staticmesh1 (`self.StaticMesh1`))
  (bind _buttonoffset (`self.ButtonOffset`))
  (bind (_relativelocation_x _relativelocation_y _relativelocation_z) (`KismetMathLibrary.BreakVector` (`SceneComponent.RelativeLocation` _staticmesh1)))
  ;[1 1 1] Button Press
  (if (`self.Press Me`)
    (`/Engine/EditorBlueprintResources/StandardMacros.DoOnce` false :!label _label
      (:`Completed`
        (set `self.Press Me` false)
        ;;[1 1 1] If true then the button moves down from its original position
        (set `self.Going Down` true)
        (`KismetSystemLibrary.MoveComponentTo` _staticmesh1 (`KismetMathLibrary.MakeVector` _relativelocation_x _relativelocation_y (+ _relativelocation_z (`KismetMathLibrary.SelectFloat` (* _buttonoffset -1.0) _buttonoffset (`self.Going Down`)))) (struct) false false 1.0 :!label _label_2)
        (if (`self.Going Down`)
          (`self.Button Pressed`)
          (set `self.Going Down` false)
          (goto _label_2)
          (else
            (goto _label :!via `Reset`)))))))

(fn `Button Pressed`
  (bind _collided_potion (`self.Collided potion`))
  (bind _book_recipies (`self.Book Recipies`))
  (`/Engine/EditorBlueprintResources/StandardMacros.IsValid` _collided_potion
    (:`Is Valid`
      ;[1 1 1] find the row
      (bind _values (`BlueprintMapLibrary.Map_Values` _book_recipies))
      ;[1 1 1] get the type of potion to change to
      (bind _keys (`BlueprintMapLibrary.Map_Keys` _book_recipies))
      (`/Game/GameItems/Potion/Potion.Change Potion` _collided_potion (`|GetArrayItem` _keys (`KismetArrayLibrary.Array_Find` _values (`|GetArrayItem` (`Actor.Tags` _collided_potion))))))))

(fn `Set Colour`
  (params (Colour :type "Color Structure"))
  (`MeshComponent.SetVectorParameterValueOnMaterials` (`self.StaticMesh`) "Colour" (`KismetMathLibrary.MakeVector` (`KismetMathLibrary.Conv_ByteToDouble` Colour_B) (`KismetMathLibrary.Conv_ByteToDouble` Colour_G) (`KismetMathLibrary.Conv_ByteToDouble` Colour_R))))

(fn `UserConstructionScript`)