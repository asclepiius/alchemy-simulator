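; BP_Cauldron is a crafting workstation that brews potions from liquids and tagged items, using Cauldron recipes loaded from a data table.
; Physics liquid balls hitting the Liquid incrementally fill their type's amount and retint it, while tagged items count as full ingredients and are destroyed.
; Tick checks recipes once all amounts are full, spawning the matched potion, or a Mundane one when no full or partial match exists.
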(event `self.ReceiveBeginPlay`
  (bind _outrownames (`DataTableFunctionLibrary.GetDataTableRowNames` "/Game/GameItems/WorkStations/RecipesTable.RecipesTable"))
  (for _array_element _outrownames
    (bind _returnvalue (`|GetDataTableRow` "/Game/GameItems/WorkStations/RecipesTable.RecipesTable" _array_element)
      (:`then`
        (if (== (`.Method_24_F3454A504680DDBA55210A8CD9D7705C` (break `/Game/GameItems/WorkStations/RecipesStruct` _returnvalue)) "Cauldron")
          (`BlueprintMapLibrary.Map_Add` (`self.Recipies`) _array_element (make `/Game/GameItems/WorkStations/Cauldron/CauldronRecipiesStruct` (break `/Game/GameItems/WorkStations/RecipesStruct` _returnvalue) (`.Crafting_Ingredient_2_33_AEBDB55D47C2DB1B056781B7B59A2FF0` (break `/Game/GameItems/WorkStations/RecipesStruct` _returnvalue)) (`.Crafting_Ingredient_3_34_C224D8244218D728AB3A5B8B437B8F74` (break `/Game/GameItems/WorkStations/RecipesStruct` _returnvalue)))))))))

(event `self.Liquid.OnComponentHit`
  (params (HitComponent :type "PrimitiveComponent Object Reference") (OtherActor :type "Actor Object Reference") (OtherComp :type "PrimitiveComponent Object Reference") (NormalImpulse :type "Vector Structure") (Hit :type "HitResult Structure (by ref)"))
  (bind _itemtag (`self.Itemtag`))
  ;[1 1 1] on collision try to cast to ball
  (if (`self.ActorHasTag` OtherActor "Potion_Liquid")
    (bind _asball_physics (cast `/Game/GameItems/Potion/BallPhysics` OtherActor))
    (bind _type (`/Game/GameItems/Potion/BallPhysics.Type` _asball_physics))
    (if (!= _type "Mundane")
      ;[1 1 1] remove liquid from potion and all to cauldren then kill the ball
      (`/Game/GameItems/Potion/BallPhysics.Remove Liquid` _asball_physics)
      (`self.Add more Liquid else Create Liquid` _type)
      (`self.ChangeColour`)
      (`/Game/GameItems/Potion/BallPhysics.Die` _asball_physics))
    (else
      (set `self.Itemtag` "None")
      ;[1 1 1] if its one of the items add it to the potion
      (for _array_element (`self.Item Tags`)
        (if (`self.ActorHasTag` OtherActor _array_element)
          (set `self.Itemtag` _array_element)))
      (if (!= _itemtag "None")
        (`self.Add Item` _itemtag)
        (`self.K2_DestroyActor` OtherActor)))))

(event `self.ReceiveTick`
  (params (DeltaSeconds :type "Float (single-precision)"))
  (bind (_returnvalue_location _returnvalue_rotation) (`KismetMathLibrary.BreakTransform` (`SceneComponent.K2_GetComponentToWorld` (`self.Potion Spawn Point`))))
  (bind (_returnvalue_location_2 _returnvalue_rotation_2) (`KismetMathLibrary.BreakTransform` (`SceneComponent.K2_GetComponentToWorld` (`self.Potion Spawn Point`))))
  ;[1 1 1] if full do the final potion check
  (`self.Are Amounts Full`
    (:`true`
      (`/Engine/EditorBlueprintResources/StandardMacros.DoOnce` false :!label _label
        (:`Completed`
          (bind __temp__current_key (`self.Check For Recipies`)
            (:`Fail`
              (if (> (`BlueprintMapLibrary.Map_Length` (`self.Added Potions `)) 0)
                (`self.Are Amounts Full`
                  (:`true`
                    ;[1 1 1] fail/mundane potion
                    (`BlueprintMapLibrary.Map_Clear` (`self.Added Potions `))
                    (bind _returnvalue (`|SpawnActorFromClass` "/Game/GameItems/Potion/Potion.Potion_C" (`KismetMathLibrary.MakeTransform` _returnvalue_location _returnvalue_rotation) "AlwaysSpawn" "MultiplyWithRoot" null null))
                    (set `/Game/GameItems/Potion/Potion.Type` "Mundane" _returnvalue)
                    ;[1 1 1] set material to green
                    (`KismetArrayLibrary.Array_Clear` (`self.Failed Recipies`) :!label _label_2)
                    (`MeshComponent.SetVectorParameterValueOnMaterials` (`self.Liquid`) "Colour" (0.45098 1.0 0.039216))))))
            (:`Success`
              (`self.Are Amounts Full`
                (:`true`
                  ;[1 1 1] One option remaining so spawn it
                  (`BlueprintMapLibrary.Map_Clear` (`self.Added Potions `))
                  (bind _returnvalue_2 (`|SpawnActorFromClass` "/Game/GameItems/Potion/Potion.Potion_C" (`KismetMathLibrary.MakeTransform` _returnvalue_location_2 _returnvalue_rotation_2) "AlwaysSpawn" "MultiplyWithRoot" null null))
                  (bind _keys (`BlueprintMapLibrary.Map_Keys` (`self.(Temp) MatchedRecipiesHolder`)))
                  (`KismetSystemLibrary.PrintString` (`KismetStringLibrary.Conv_NameToString` __temp__current_key))
                  (set `/Game/GameItems/Potion/Potion.Type` __temp__current_key _returnvalue_2)
                  (goto _label_2))))))))
    (:`false`
      (goto _label :!via `Reset`))))

(fn `ChangeColour`
  (bind _values (`BlueprintMapLibrary.Map_Values` (`self.Added Potions `)))
  (set `self.ColourVal` (1.0 1.0 1.0))
  (for _array_element _values
    (set `self.ColourVal` (* (* (break `/Game/GameItems/WorkStations/Cauldron/CauldonStruct` _array_element) (/ (`.Amount_9_DCF26FD94B286CFC4C1E0AA75513E767` (break `/Game/GameItems/WorkStations/Cauldron/CauldonStruct` _array_element)) 100.0)) (`self.ColourVal`))))
  (`MeshComponent.SetVectorParameterValueOnMaterials` (`self.Liquid`) "Colour" (`self.ColourVal`)))

(fn `Check`
  (params (Recipie :type "Array of Name (by ref)") (`Added Ingredient` :type Name))
  (returns (`type out` :type Integer))
  (bind _returnvalue (!= (`KismetArrayLibrary.Array_Find` Recipie `Added Ingredient`) -1))
  (if _returnvalue
    (return 2)
    (elif _returnvalue
      (return 1)
      (else
        (return 0)))))

(fn `Check Recipies`
  (returns (NewParam :type Integer))
  ;[1 1 1] loops for each value in map and sets temp variables
  (`BlueprintMapLibrary.Map_Clear` (`self.(Temp) MatchedRecipiesHolder`))
  (set `self.Did Find` false)
  (`self.For each value set temp` (`self.Recipies`)
    (:`Loop`
      (set `self.(Temp) Is valid Recipie` true)
      ;[1 1 1] goes through every ingredient that has been added and checks there is a valid combo
      (bind _keys (`BlueprintMapLibrary.Map_Keys` (`self.Added Potions `)))
      (for _array_element (`self.(Temp) Recipie`)
        (`self.Check if in recipie` _keys _array_element))
      ;[1 1 1] add recipie if its valid
      (if (`self.(Temp) Is valid Recipie`)
        (`BlueprintMapLibrary.Map_Add` (`self.(Temp) MatchedRecipiesHolder`) (`self.Key`) (`self.(Temp) Current Ingredients`))
        (set `self.Did Find` true)))
    (:`Completed`
      (switch `int` (`KismetMathLibrary.Clamp` (`BlueprintMapLibrary.Map_Length` (`self.(Temp) MatchedRecipiesHolder`)) 0 2)))))

(fn `UserConstructionScript`)